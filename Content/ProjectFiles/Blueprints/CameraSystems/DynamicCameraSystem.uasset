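; Level-placed dynamic camera that takes over the player's view via an enable trigger and hands it back to the character via a disable trigger, using blended view target switches.
; While active, Tick either turns a stationary camera toward the player or moves the spring arm with them.
; Movement uses the TrackPlayer vector as a per-axis mask between player location and the camera actor's location minus an offset set on first activation.
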(event `self.Enable Camera.OnComponentBeginOverlap`
  (params (OverlappedComponent :type "PrimitiveComponent Object Reference") (OtherActor :type "Actor Object Reference") (OtherComp :type "PrimitiveComponent Object Reference") (OtherBodyIndex :type Integer) (bFromSweep :type Boolean) (SweepResult :type "HitResult Structure (by ref)"))
  (cast `/Game/ProjectFiles/Blueprints/CharacterLogic/MyCharacterBP` OtherActor)
  (`self.Switch Camera To New View Target` self
    (:`Exec`
      (`/Engine/EditorBlueprintResources/StandardMacros.DoOnce` false
        (:`Completed`
          (set `self.Offset` (- (`SceneComponent.K2_GetComponentLocation` (`self.SpringArm`)) (`self.K2_GetActorLocation` (`GameplayStatics.GetPlayerCharacter` 0)))))))))

(event `self.Disable Camera.OnComponentBeginOverlap`
  (params (OverlappedComponent :type "PrimitiveComponent Object Reference") (OtherActor :type "Actor Object Reference") (OtherComp :type "PrimitiveComponent Object Reference") (OtherBodyIndex :type Integer) (bFromSweep :type Boolean) (SweepResult :type "HitResult Structure (by ref)"))
  (bind _asmy_character_bp (cast `/Game/ProjectFiles/Blueprints/CharacterLogic/MyCharacterBP` OtherActor))
  (`self.Switch Camera To New View Target` _asmy_character_bp))

(event `self.ReceiveTick`
  (params (DeltaSeconds :type "Float (single-precision)"))
  (if (== (`Controller.GetViewTarget` (`GameplayStatics.GetPlayerController` 0)) self)
    (if (`self.IsStationary`)
      (bind _rotation (`self.TrackPlayerRotation` DeltaSeconds))
      (`SceneComponent.K2_SetWorldRotation` (`self.Camera`) _rotation false false)
      (else
        (bind _vector (`self.TrackPlayerMovement` DeltaSeconds))
        (`SceneComponent.K2_SetWorldLocation` (`self.SpringArm`) _vector false false)))))

(fn `TrackPlayerMovement`
  (params (`Delta Time` :type "Float (double-precision)"))
  (returns (Vector :type "Vector Structure"))
  (bind _returnvalue (- (`self.K2_GetActorLocation`) (`self.Offset`)))
  (return (`KismetMathLibrary.VInterpTo` _returnvalue (+ (* _returnvalue (- (1.0 1.0 1.0) (`self.TrackPlayer`))) (* (`self.K2_GetActorLocation` (`GameplayStatics.GetPlayerCharacter` 0)) (`self.TrackPlayer`))) `Delta Time`)))

(fn `TrackPlayerRotation`
  (params (`Delta Time` :type "Float (double-precision)"))
  (returns (Rotation :type "Rotator Structure"))
  (return (`KismetMathLibrary.FindLookAtRotation` (`SceneComponent.K2_GetComponentLocation` (`self.Camera`)) (`self.K2_GetActorLocation` (`GameplayStatics.GetPlayerCharacter` 0)))))

(fn `UserConstructionScript`)